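; Actor that spawns enemy elephants around itself, capped at three tracked at once.
; Spawn places an LPElephant at a random nearby XY offset at zero height, tags it Enemy, enables patrol and attack, and randomizes its level.
; A looping BeginPlay timer runs ValidCheck to prune invalid entries from ElephantArray.
; The random-interval timer that would call Spawn is disconnected, so nothing in this Blueprint triggers spawning.
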(event `self.ReceiveBeginPlay`
  (`KismetSystemLibrary.K2_SetTimer` null "ValidCheck" 0.5 true))

(event `self.ReceiveActorBeginOverlap`
  (params (OtherActor :type "Actor Object Reference")))

(fn `Spawn`
  (bind _returnvalue (`KismetMathLibrary.RandomFloatInRange` -1000.0 1000.0))
  (if (< (`KismetArrayLibrary.Array_Length` (`self.ElephantArray`)) 3)
    (bind _returnvalue_2 (`|SpawnActorFromClass` "/Script/LionProject.LPElephant" (`KismetMathLibrary.MakeTransform` (`KismetMathLibrary.MakeVector` (+ (.x (.location (`self.GetTransform`))) _returnvalue) (+ (.y (.location (`self.GetTransform`))) _returnvalue)) (.rotation (`self.GetTransform`)) (.scale (`self.GetTransform`))) "Undefined" "OverrideRootScale" null null))
    (`/Engine/EditorBlueprintResources/StandardMacros.IsValid` _returnvalue_2
      (:`Is Valid`
        (`KismetArrayLibrary.Array_Add` (`Actor.Tags` _returnvalue_2) "Enemy")
        (`LPAnimal.SetIsPatrol` _returnvalue_2 true)
        (`LPAnimal.SetIsAttack` _returnvalue_2 true)
        (bind _returnvalue_3 (`LPAnimal.GetLPPlayerState` _returnvalue_2))
        (`LPPlayerState.SetCharacterLevel` _returnvalue_3 (`KismetMathLibrary.RandomIntegerInRange` 10 15))
        (`KismetArrayLibrary.Array_Add` (`self.ElephantArray`) _returnvalue_2)))))

(fn `UserConstructionScript`)

(fn `ValidCheck`
  (for _array_element (`self.ElephantArray`)
    (`/Engine/EditorBlueprintResources/StandardMacros.IsValid` _array_element
      (:`Is Not Valid`
        (`KismetArrayLibrary.Array_RemoveItem` (`self.ElephantArray`) _array_element)))))