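; KillZVolume_BP is a kill volume that removes certain actors when they begin overlapping it.
; The overlap event ignores player 0's pawn and destroys any LPAnimal together with its LPPlayerState.
; Other actors are destroyed only if they carry the "Log" tag.
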(event `self.ReceiveActorBeginOverlap`
  (params (OtherActor :type "Actor Object Reference"))
  (if (not (== OtherActor (`GameplayStatics.GetPlayerPawn` 0)))
    (bind _aslpanimal (cast `LPAnimal` OtherActor)
      (:`then`
        (`/Engine/EditorBlueprintResources/StandardMacros.IsValid` _aslpanimal
          (:`Is Valid`
            (bind _returnvalue (`LPAnimal.GetLPPlayerState` _aslpanimal))
            (`self.K2_DestroyActor` _returnvalue)
            (`self.K2_DestroyActor` _aslpanimal))))
      (:`CastFailed`
        (if (`self.ActorHasTag` OtherActor "Log")
          (`/Engine/EditorBlueprintResources/StandardMacros.IsValid` OtherActor
            (:`Is Valid`
              (`self.K2_DestroyActor` OtherActor))))))))

(fn `UserConstructionScript`)