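; Plasma bolt actor, named as an ultimate attack, that damages the player on overlap.
; When the overlapping actor is player pawn 0 and casts to LPLionBaby, it applies random damage within a fixed high range.
; Only the overlap event has logic, and it calls the parent's handler first.
; The bolt defines no movement or destruction in this graph.
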(event `self.ReceiveActorBeginOverlap`
  (params (OtherActor :type "Actor Object Reference"))
  (`parent.ReceiveActorBeginOverlap` OtherActor)
  (if (== OtherActor (`GameplayStatics.GetPlayerPawn` 0))
    (bind _aslplion_baby (cast `LPLionBaby` (`GameplayStatics.GetPlayerPawn` 0)))
    (`GameplayStatics.ApplyDamage` _aslplion_baby (`KismetMathLibrary.RandomFloatInRange` 80.0 160.0))))

(fn `UserConstructionScript`
  (`parent.UserConstructionScript`))