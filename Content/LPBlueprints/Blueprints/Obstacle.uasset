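; Obstacle actor that drifts in a straight line along MovementDirection while spinning, with each instance varying in size, speed and rotation.
; The construction script randomizes the RotatingMovement rotation rate without roll, a uniform scale, and CurrentSpeed, using min/max variables for scale and speed.
; Tick applies a delta-time-scaled world offset without sweep, so movement passes through blockers.
; BeginPlay and overlap events are empty.
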(event `self.ReceiveTick`
  (params (DeltaSeconds :type "Float (single-precision)"))
  (`self.K2_AddActorWorldOffset` (* (`self.MovementDirection`) (* DeltaSeconds (`self.CurrentSpeed`)))))

(fn `UserConstructionScript`
  (set `RotatingMovementComponent.RotationRate` (`KismetMathLibrary.RandomRotator` false) (`self.RotatingMovement`))
  (`self.SetActorScale3D` (`KismetMathLibrary.Conv_DoubleToVector` (`KismetMathLibrary.RandomFloatInRange` (`self.RandomScaleMin`) (`self.RandomScaleMax`))))
  (set `self.CurrentSpeed` (`KismetMathLibrary.RandomFloatInRange` (`self.SpeedMin`) (`self.SpeedMax`))))