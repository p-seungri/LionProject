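; LogSpawner_BP is a spawner actor that periodically creates LPFloatingLog actors.
; Five seconds after BeginPlay, it starts a looping timer on Spawn, with an interval randomized only once between MinTime and MaxTime.
; Each log takes the spawner's XY, rotation and scale at a hardcoded Z height, gets a "Log" tag and receives a random speed between MinSpeed and MaxSpeed.
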(event `self.ReceiveBeginPlay`
  (`KismetSystemLibrary.Delay` 5.0)
  (`KismetSystemLibrary.K2_SetTimer` null "Spawn" (`KismetMathLibrary.RandomFloatInRange` (`self.MinTime`) (`self.MaxTime`)) true))

(fn `Spawn`
  (bind _returnvalue (`|SpawnActorFromClass` "/Script/LionProject.LPFloatingLog" (`KismetMathLibrary.MakeTransform` (`KismetMathLibrary.MakeVector` (.x (.location (`self.GetTransform`))) (.y (.location (`self.GetTransform`))) -125.0) (.rotation (`self.GetTransform`)) (.scale (`self.GetTransform`))) "Undefined" "OverrideRootScale" null null))
  (`KismetArrayLibrary.Array_Add` (`Actor.Tags` _returnvalue) "Log")
  (set `LPFloatingLog.CurrentSpeed` (`KismetMathLibrary.RandomFloatInRange` (`self.MinSpeed`) (`self.MaxSpeed`)) _returnvalue))

(fn `UserConstructionScript`)